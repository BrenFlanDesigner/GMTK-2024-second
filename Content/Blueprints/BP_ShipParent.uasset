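; Parent Blueprint for ships, providing movement, projectile firing, health and size-scaled damage.
; Start/End events play and stop Timelines that apply forward or half-strength reverse input along ShipArrow each update, or yaw player controller 0's control rotation to turn.
; FireProjectile spawns ProjectileClass at the arrow.
; ConveyDamage scales base damage by attacker-to-victim size ratio, passes it to ACHealth and calls the empty Die when that returns true.
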(event `ThrustStart`
  ;[1 1 1] Basic Ship Controls
  ;;[1 0 0.01123] Thrust. Apply constant thrust when active, stop when stopped
  (`Timeline|Timeline_1` :!label _label
    (:`Update`
      (`self.AddMovementInput` (`SceneComponent.GetForwardVector` (`self.ShipArrow`))))))

(event `ThrustEnd`
  ;[1 1 1] Basic Ship Controls
  ;;[1 0 0.01123] Thrust. Apply constant thrust when active, stop when stopped
  (goto _label :!via `Stop`))

(event `ReverseStart`
  ;[1 1 1] Basic Ship Controls
  ;;[0 0.3398 1] Reverse
  (`Timeline|Timeline_0` :!label _label_2
    (:`Update`
      (`self.AddMovementInput` (`SceneComponent.GetForwardVector` (`self.ShipArrow`)) -0.5))))

(event `ReverseEnd`
  ;[1 1 1] Basic Ship Controls
  ;;[0 0.3398 1] Reverse
  (goto _label_2 :!via `Stop`))

(event `TurnStart`
  (params (`Left?` :type Boolean))
  (bind (_returnvalue_roll _returnvalue_pitch _returnvalue_yaw) (`KismetMathLibrary.BreakRotator` (`self.GetControlRotation`)))
  ;[1 1 1] Basic Ship Controls
  ;;[0 1 0.2649] Turning
  (`Timeline|Timeline` :!label _label_3
    (:`Update`
      (`Controller.SetControlRotation` (`GameplayStatics.GetPlayerController` 0) (`KismetMathLibrary.MakeRotator` _returnvalue_roll _returnvalue_pitch (+ _returnvalue_yaw (* (`KismetMathLibrary.SelectFloat` -1.0 1.0 `Left?`) (`self.TurnSpeed`))))))))

(event `TurnEnd`
  ;[1 1 1] Basic Ship Controls
  ;;[0 1 0.2649] Turning
  (goto _label_3 :!via `Stop`))

(event `FireProjectile`
  (bind _shiparrow (`self.ShipArrow`))
  ;[1 1 1] Basic Ship Controls
  (`|SpawnActorFromClass` (`self.ProjectileClass`) (`KismetMathLibrary.MakeTransform` (`SceneComponent.K2_GetComponentLocation` _shiparrow) (`SceneComponent.K2_GetComponentRotation` _shiparrow)) "Undefined" "MultiplyWithRoot" self self))

(event `SetMaxHealth`
  (`/Game/Blueprints/AC_Health.InitializeMaxHealth` (`self.AC_Health`)))

(event `SetShipSize`
  (params (NewShipSize :type Integer))
  (set `self.ShipSize` NewShipSize))

(fn `ConveyDamage`
  (params (InstigatorShipSize :type Integer))
  (returns (`bIsDead?` :type Boolean))
  (bind _returnvalue (`KismetMathLibrary.Conv_IntToDouble` InstigatorShipSize))
  (bind _shipsize (`self.ShipSize`))
  (bind _returnvalue_2 (* (/ _returnvalue (`KismetMathLibrary.Conv_IntToDouble` _shipsize)) (`self.BaseDamageValue`)))
  (`KismetSystemLibrary.PrintString` (`KismetStringLibrary.Concat_StrStr` "Damage Event: Attacking Ship Size : " (`KismetStringLibrary.Conv_DoubleToString` _returnvalue) "Hit Ship Size: " (`KismetStringLibrary.Conv_IntToString` _shipsize) "      Damage Conveyed: " (`KismetStringLibrary.Conv_DoubleToString` _returnvalue_2)))
  (bind _bisdead (`/Game/Blueprints/AC_Health.TakeDamage1` (`self.AC_Health`) _returnvalue_2))
  (if _bisdead
    (`self.Die`))
  (return _bisdead))

(fn `Die`)

(fn `UserConstructionScript`)