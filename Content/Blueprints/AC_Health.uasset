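; Health component that tracks current health, maximum health and death state for an actor, expected to be a BP_ShipParent.
; On BeginPlay it caches its owner as that ship type.
; AddHealth caps healing at the maximum, while TakeDamage1 subtracts damage, clamps at zero, sets IsDead and returns whether the hit was lethal.
; InitializeMaxHealth is an empty event.
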(event `InitializeMaxHealth`)

(event `self.ReceiveBeginPlay`
  (bind _asbp_ship_parent (cast `/Game/Blueprints/BP_ShipParent` (`self.GetOwner`)))
  (set `self.OwningActor` _asbp_ship_parent))

(event `AddHealth`
  (params (HealValue :type "Float (double-precision)"))
  (bind _returnvalue (+ HealValue (`self.CurrentHealth`)))
  (if (>= _returnvalue (`self.MaxHealth`))
    (set `self.CurrentHealth` (`self.MaxHealth`))
    (else
      (set `self.CurrentHealth` _returnvalue))))

(fn `TakeDamage1`
  (params (DamageValue :type "Float (double-precision)"))
  (returns (bIsDead :type Boolean))
  (bind _returnvalue (- (`self.CurrentHealth`) DamageValue))
  (if (<= _returnvalue 0.0)
    (set `self.bIsDead` true)
    (set `self.CurrentHealth` 0.0)
    (return true)
    (else
      (set `self.CurrentHealth` _returnvalue)
      (return false))))