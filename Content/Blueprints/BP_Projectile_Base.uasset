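; Base projectile Blueprint that delivers damage on behalf of the ship that owns it.
; On BeginPlay it casts its owner to BP_ShipParent and stores it as OwningShip.
; When HitBox overlaps an actor of a different class from the owning ship, a DoOnce lets it call ConveyDamageMessage once, passing the owner's ShipSize.
; Actors of the owner's exact class are ignored.
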(event `self.ReceiveBeginPlay`
  (bind _asbp_ship_parent (cast `/Game/Blueprints/BP_ShipParent` (`self.GetOwner`)))
  (set `self.OwningShip` _asbp_ship_parent))

(event `self.HitBox.OnComponentBeginOverlap`
  (params (OverlappedComponent :type "PrimitiveComponent Object Reference") (OtherActor :type "Actor Object Reference") (OtherComp :type "PrimitiveComponent Object Reference") (OtherBodyIndex :type Integer) (bFromSweep :type Boolean) (SweepResult :type "HitResult Structure (by ref)"))
  (bind _owningship (`self.OwningShip`))
  (if (!= (`GameplayStatics.GetObjectClass` OtherActor) (`GameplayStatics.GetObjectClass` _owningship))
    (`/Engine/EditorBlueprintResources/StandardMacros.DoOnce` false
      (:`Completed`
        (message `/Game/Blueprints/BPI_Combat.ConveyDamage` OtherActor (`/Game/Blueprints/BP_ShipParent.ShipSize` _owningship))))))

(fn `UserConstructionScript`)