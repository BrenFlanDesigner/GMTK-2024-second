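; Spawner actor that periodically activates enemy ships from an object pool around its own location.
; A looping timer takes the first unspawned ship in EnemyObjectPool, teleports it to a random horizontal offset and spawns it.
; Ship size is ShipsSpawned divided by three, so it climbs as the counter rises on each timer tick, even when no pooled ship is free.
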(event `self.ReceiveBeginPlay`
  (`KismetSystemLibrary.K2_SetTimer` null "SpawnShip" (`self.SpawnTimer`) true))

(event `SpawnShip`
  (bind _shiptospawn (`self.ShipToSpawn`))
  (for _array_element (`self.EnemyObjectPool`) :!label _label
    (if (not (`/Game/Blueprints/BP_Ship_Enemy.Spawned` _array_element))
      (set `self.ShipToSpawn` _array_element)
      (`self.BreakLoop`)
      (`self.K2_SetActorLocation` _shiptospawn (+ (`self.K2_GetActorLocation` self) (`KismetMathLibrary.MakeVector` (`KismetMathLibrary.RandomFloatInRange` -500.0 500.0) (`KismetMathLibrary.RandomFloatInRange` -500.0 500.0))) false true)
      (bind _output_get (set `self.ShipSizeToSpawn` (/ (`self.ShipsSpawned`) 3)))
      (`/Game/Blueprints/BP_ShipParent.SetShipSize` _shiptospawn _output_get)
      (`/Game/Blueprints/BP_Ship_Enemy.Spawn` _shiptospawn)
      (`KismetSystemLibrary.PrintString` (`KismetStringLibrary.Concat_StrStr` "SpawnedShip Size:  " (`KismetStringLibrary.Conv_IntToString` _output_get)))))
  (`/Engine/EditorBlueprintResources/StandardMacros.IncrementInt` (`self.ShipsSpawned`)))

(event `BreakLoop`
  (goto _label :!via `Break`))

(fn `UserConstructionScript`)