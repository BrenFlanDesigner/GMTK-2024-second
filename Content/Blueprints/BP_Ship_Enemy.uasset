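; BP_Ship_Enemy is an enemy ship that is hidden and reused instead of destroyed.
; It despawns on BeginPlay and after the parent Die logic, hiding its mesh, clearing Spawned and teleporting to a fixed off-field location.
; Spawn reveals the mesh, sets Spawned and resets health, leaving positioning to other code.
; Thrust and Shoot events wrap timed thrust and projectile fire, with no decision logic in this Blueprint.
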(event `self.ReceiveBeginPlay`
  (`self.Despawn`))

(event `Despawn`
  (`SceneComponent.SetHiddenInGame` (`self.ShipMesh`) true false)
  (set `self.Spawned` false)
  (`self.K2_SetActorLocation` (0.0 0.0 10000.0) false true))

(event `Spawn`
  (`SceneComponent.SetHiddenInGame` (`self.ShipMesh`) false false)
  (set `self.Spawned` true)
  (`self.SetMaxHealth`))

(event `/Game/Blueprints/BPI_EnemyShipFunctions.Thrust`
  (params (ThrustDuration :type "Float (double-precision)"))
  (`self.ThrustStart`)
  (`KismetSystemLibrary.Delay` ThrustDuration)
  (`self.ThrustEnd`))

(event `/Game/Blueprints/BPI_EnemyShipFunctions.Shoot`
  (`self.FireProjectile`))

(fn `Die`
  (`parent.Die`)
  (`self.Despawn`))

(fn `UserConstructionScript`
  (`parent.UserConstructionScript`))