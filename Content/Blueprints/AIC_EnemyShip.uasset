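; AI controller for an enemy ship that attacks whatever its perception senses.
; When a target is sensed, it sets focus on it, sends a full thrust message to the pawn and starts a looping Fire timer at the fire rate.
; Each Fire tick sends a shoot message to the pawn.
; Losing the target clears focus and stops the timer, with no message to stop thrust.
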(event `self.AIPerception.OnTargetPerceptionUpdated`
  (params (Actor :type "Actor Object Reference") (Stimulus :type "AIStimulus Structure"))
  (if (`.bSuccessfullySensed` (break `AIStimulus` Stimulus))
    (`self.K2_SetFocus` Actor)
    (message `/Game/Blueprints/BPI_EnemyShipFunctions.Thrust` (`self.K2_GetPawn`) 1.0)
    (bind _returnvalue (`KismetSystemLibrary.K2_SetTimer` null "Fire" (`self.FireRate`) true))
    (set `self.FireTimer` _returnvalue)
    (else
      (`self.K2_ClearFocus`)
      (`KismetSystemLibrary.K2_ClearAndInvalidateTimerHandle` (`self.FireTimer`)))))

(event `Fire`
  (message `/Game/Blueprints/BPI_EnemyShipFunctions.Shoot` (`self.K2_GetPawn`)))

(fn `UserConstructionScript`)